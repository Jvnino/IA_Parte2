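; AI controller for a soldier that patrols between randomly chosen waypoints.
; On BeginPlay it gathers every BP_Waypoint whose AICharacter list holds the controlled AI_Character, shuffles Routes and moves to the first entry.
; Each completed move, whatever its result, waits briefly and repeats the gathering, appending to Routes without clearing it, so the same waypoint can be picked again.
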(event `self.ReceiveBeginPlay`
  (bind _routes (`self.Routes`))
  ;[1 1 1] Movimiento de waypoints
  (add `self.ReceiveMoveCompleted` (delegate `ReceiveMoveCompleted_Event`))
  (bind _outactors (`GameplayStatics.GetAllActorsOfClass` "/Game/Blueprints/BP_Waypoint.BP_Waypoint_C" :!label _label))
  (bind _asai_character (cast `/Game/Blueprints/AI_Character` (`self.K2_GetPawn`)))
  (for _array_element _outactors
    (if (!= (`KismetArrayLibrary.Array_Find` (`/Game/Blueprints/BP_Waypoint.AI_Character` _array_element) _asai_character) -1)
      (`KismetArrayLibrary.Array_Add` (`self.Routes`) _array_element)))
  (`KismetArrayLibrary.Array_Shuffle` _routes)
  (`self.MoveToActor` (`|GetArrayItem` _routes) -1.0 true true true null))

(event `ReceiveMoveCompleted_Event` :!signature `self.ReceiveMoveCompleted`
  (params (RequestID :type "AIRequestID Structure") (Result :type "EPathFollowingResult Enum" :default "Success"))
  ;[1 1 1] Movimiento de waypoints
  (`KismetSystemLibrary.Delay` 1.0)
  (goto _label))

(fn `UserConstructionScript`)